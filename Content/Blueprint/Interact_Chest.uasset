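; Interactable chest Blueprint whose lid opens and closes on alternating interactions.
; On BeginPlay it copies the Block mesh's first material onto the chest top mesh.
; Interact flip-flops between playing the OpenChest timeline from the start and reversing it, with the timeline driving the pitch of a Rotator component to swing the lid.
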(event `self.ReceiveBeginPlay`
  (`parent.ReceiveBeginPlay`)
  (`PrimitiveComponent.SetMaterial` (`self.SM_Chest_Top`) 0 (`PrimitiveComponent.GetMaterial` (`self.Block`) 0)))

(event `self.Interact`
  (`/Engine/EditorBlueprintResources/StandardMacros.FlipFlop`
    (:`A`
      (bind (_direction _newtrack_0) (`Timeline|OpenChest` :!via `PlayFromStart` :!label _label)
        (:`Update`
          (`SceneComponent.K2_SetRelativeRotation` (`self.Rotator`) (`KismetMathLibrary.MakeRotator` 0.0 _newtrack_0) false false))))
    (:`B`
      (goto _label :!via `Reverse`))))

(fn `UserConstructionScript`
  (`parent.UserConstructionScript`))