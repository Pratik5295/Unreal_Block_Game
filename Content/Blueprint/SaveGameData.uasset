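; SaveGameData is a data container for saved game state: player position, Wood and Stone amounts, and the game's blocks.
; Paired setter and getter functions write and return the player details together, while the blocks have their own pair.
; AddBlocks replaces the stored Blocks with the passed value rather than appending to it.
; The functions only assign or return variables, with no slot save or load calls.
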(fn `AddBlocks`
  (params (GameBlocks :type "Map of Transform Structure to /Game/Blueprint/BP_Block Class Reference"))
  (set `self.Blocks` GameBlocks))

(fn `Get Player Details`
  (returns (`Player Position` :type "Vector Structure") (Wood :type Integer) (Stone :type Integer))
  (return (`self.PlayerPosition`) (`self.Wood`) (`self.Stone`)))

(fn `GetBlocksData`
  (returns (`Saved Blocks` :type "Map of Transform Structure to /Game/Blueprint/BP_Block Class Reference"))
  (return (`self.Blocks`)))

(fn `Save Player Details`
  (params (PlayerPos :type "Vector Structure") (Wood :type Integer) (Stone :type Integer))
  (set `self.PlayerPosition` PlayerPos)
  (set `self.Stone` Stone)
  (set `self.Wood` Wood))