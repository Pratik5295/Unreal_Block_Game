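; Block actor that can be gradually destroyed, with its material showing the progress.
; BeginPlay creates a dynamic material instance on the Block component and sets the destroy timeline's play rate.
; StartDestroy plays the timeline, driving the DestroyAmount parameter each update and destroying the actor when finished.
; StopDestroy zeroes the parameter and stops the timeline without rewinding it, so a later start resumes from the stopped position.
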(event `self.ReceiveBeginPlay`
  (bind _block (`self.Block`))
  (bind _returnvalue (`PrimitiveComponent.CreateDynamicMaterialInstance` _block 0 (`PrimitiveComponent.GetMaterial` _block 0) "None"))
  (bind _output_get (set `self.BlockMat` _returnvalue))
  (`TimelineComponent.SetPlayRate` (`self.DestroyTimeline`) (`self.DestroyPlayRate`)))

(event `StartDestroy`
  (bind (_direction _destroyamount) (`Timeline|DestroyTimeline` :!label _label)
    (:`Update`
      (`MaterialInstanceDynamic.SetScalarParameterValue` (stale `self.ReceiveBeginPlay` _output_get) "DestroyAmount" _destroyamount))
    (:`Finished`
      (`self.K2_DestroyActor`))))

(event `StopDestroy`
  (bind _output_get (set `self.NewVar` (stale `self.ReceiveBeginPlay` _returnvalue)))
  (`MaterialInstanceDynamic.SetScalarParameterValue` _output_get "DestroyAmount" 0.0)
  (goto _label :!via `Stop`))

(fn `UserConstructionScript`)